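; Player character Blueprint with axis-driven movement along capsule forward and right vectors, plus a tap-based dash and dodge.
; A DoubleTap macro fires Dash on the first press without waiting, and Dodge on a second press within the threshold.
; Both launch the character along scaled current velocity.
; Only the stronger Dodge toggles invincibility and blocks further dashing and dodging, setting timers for the i-frame window and recovery.
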(event `InputAxis|MoveForward`
  (params (AxisValue :type "Float (single-precision)"))
  (`self.MoveForward` AxisValue))

(event `InputAxis|MoveRight`
  (params (AxisValue :type "Float (single-precision)"))
  (`self.MoveRight` AxisValue))

(event `InputAction|Dodge`
  (params (Key :type "Key Structure"))
  (:`Pressed`
    (if (`self.CanDashDodge`)
      (`self.DoubleTap` :!label _label
        (:`Single Tap`
          (`self.Dash`))
        (:`Double Tap`
          (`self.Dodge`)))
      (else
        (`KismetSystemLibrary.PrintString` "Can't dash: too tired!"))))
  (:`Released`
    (goto _label :!via `Released`)))

(fn `Dash`
  (`self.LaunchCharacter` (* (`self.GetVelocity`) (5.0 5.0 5.0)) true true))

(fn `Dodge`
  (`self.HandleIFrames`)
  (`self.LaunchCharacter` (* (`self.GetVelocity`) (10.0 10.0 10.0)) true true)
  (`KismetSystemLibrary.K2_SetTimerDelegate` (`|CreateDelegate` :!event `HandleIFrames`) (`self.IFrameWindow`))
  (set `self.CanDashDodge` false)
  (`KismetSystemLibrary.K2_SetTimerDelegate` (`|CreateDelegate` :!event `ResetDash`) (`self.DashRecovery`)))

(fn `HandleIFrames`
  (if (`self.IsInvinsible`)
    (`KismetSystemLibrary.PrintString` "F : Invisible")
    (set `self.IsInvinsible` false)
    (else
      (`KismetSystemLibrary.PrintString` "T : Invisible")
      (set `self.IsInvinsible` true))))

(fn `MoveForward`
  (params (MovementValue :type "Float (double-precision)"))
  (`self.AddMovementInput` (`SceneComponent.GetForwardVector` (`self.CapsuleComponent`)) (* MovementValue (`self.MoveMultiplyer`) (`GameplayStatics.GetWorldDeltaSeconds`))))

(fn `MoveRight`
  (params (MovementValue :type "Float (double-precision)"))
  (`self.AddMovementInput` (`SceneComponent.GetRightVector` (`self.CapsuleComponent`)) (* MovementValue (`self.MoveMultiplyer`) (`GameplayStatics.GetWorldDeltaSeconds`))))

(fn `ResetDash`
  (set `self.CanDashDodge` true)
  (`KismetSystemLibrary.PrintString` "Dash Reset"))

(fn `UserConstructionScript`)